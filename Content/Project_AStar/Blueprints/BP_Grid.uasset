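; Grid actor that previews a tile layout with ground and obstacle detection, drawn entirely as debug shapes in the construction script.
; It flushes old lines, draws the extent box and bottom-left corner, then derives tile counts from GridSizeWorld and TileSize, both treated as half-extents.
; DrawTiles sphere-traces each tile center on two custom channels: tiles without ground are skipped, and obstacle hits change the plane color.
; No tile data is stored.
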(fn `DrawTiles`
  (bind _scene (`self.Scene`))
  (bind _tilesize (`self.TileSize`))
  (bind _returnvalue (`KismetSystemLibrary.MakeLiteralDouble` (* (`self.TileSize`) (`self.SphereTracePercentage`))))
  (bind _buttonleftcornerposition (`self.GetBottomLeft`))
  (bind (_horizontaltiles _verticaltiles) (`self.GetNumberOfTiles`))
  (for _index (range _horizontaltiles)
    (for _index_2 (range _verticaltiles)
      (bind _returnvalue_2 (+ (+ (* (`SceneComponent.GetForwardVector` _scene) (* _index_2 (`self.TileSize`) 2.0)) (`KismetMathLibrary.MakeVector` _tilesize)) (+ (* (`SceneComponent.GetRightVector` _scene) (* _index (`self.TileSize`) 2.0)) (`KismetMathLibrary.MakeVector` 0.0 _tilesize)) _buttonleftcornerposition))
      ;[1 1 1] Try Detect Ground (Only show if there is Ground)
      (bind (_outhit _returnvalue_3) (`KismetSystemLibrary.SphereTraceSingle` _returnvalue_2 (+ _returnvalue_2 (0.0 0.0 -0.01)) _returnvalue "TraceTypeQuery3"))
      (if _returnvalue_3
        ;[1 1 1] Try Detect Obstacle (Don't show if there is obstacle
        (bind (_outhit_2 _returnvalue_4) (`KismetSystemLibrary.SphereTraceSingle` _returnvalue_2 (+ _returnvalue_2 (0.0 0.0 -0.01)) _returnvalue "TraceTypeQuery4"))
        (`KismetSystemLibrary.DrawDebugPlane` (make `Plane` (.z _returnvalue_2) 0.0 0.0 1.0) _returnvalue_2 (- (`self.TileSize`) (`self.PaddingSize`)) (`KismetMathLibrary.SelectColor` (struct :`R` 0.119792 :`G` 0.03155 :`A` 1.0) (struct :`R` 1.0 :`G` 0.688256 :`A` 1.0) _returnvalue_4) 10000.0)))))

(fn `GetBottomLeft`
  (returns (ButtonLeftCornerPosition :type "Vector Structure"))
  (bind (_gridsizeworld_x _gridsizeworld_y) (`KismetMathLibrary.BreakVector2D` (`self.GridSizeWorld`)))
  (bind _scene (`self.Scene`))
  (return (- (- (`SceneComponent.K2_GetComponentLocation` (`self.Scene`)) (* (`SceneComponent.GetRightVector` _scene) _gridsizeworld_x)) (* (`SceneComponent.GetForwardVector` _scene) _gridsizeworld_y))))

(fn `GetNumberOfTiles`
  (returns (HorizontalTiles :type Integer) (VerticalTiles :type Integer))
  (bind (_gridsizeworld_x _gridsizeworld_y) (`KismetMathLibrary.BreakVector2D` (`self.GridSizeWorld`)))
  (bind _tilesize (`self.TileSize`))
  (return (`KismetMathLibrary.FFloor` (/ _gridsizeworld_x _tilesize)) (`KismetMathLibrary.FFloor` (/ _gridsizeworld_y _tilesize))))

(fn `UserConstructionScript`
  (bind (_gridsizeworld_x _gridsizeworld_y) (`KismetMathLibrary.BreakVector2D` (`self.GridSizeWorld`)))
  (`KismetSystemLibrary.FlushPersistentDebugLines`)
  (bind _output_get (set `self.GridLocation` (`SceneComponent.K2_GetComponentLocation` (`self.Scene`))))
  ;[0 0.2421 1] Draw Extent Box
  (`KismetSystemLibrary.DrawDebugBox` _output_get (`KismetMathLibrary.MakeVector` _gridsizeworld_y _gridsizeworld_x) (`self.GridColor`) (struct) 1000000.0 10.0)
  ;[1 0.07005 0.8238] Draw Debug Box in BottomLeftCorner
  (bind _buttonleftcornerposition (`self.GetBottomLeft`))
  (`KismetSystemLibrary.DrawDebugSphere` _buttonleftcornerposition 10.0 8 (struct :`R` 1.0 :`B` 0.949276 :`A` 1.0) 10000.0 10.0)
  ;[1 0.9804 0] Draw Tiles
  (`self.DrawTiles`))