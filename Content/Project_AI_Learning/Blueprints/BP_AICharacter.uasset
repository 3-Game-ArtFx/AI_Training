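; AI character Blueprint that switches to rifle combat when an enemy is found and leaves it when the enemy is lost.
; Finding an enemy opens a Gate that loops through a retriggerable delay, calling FireBullet after a short delay while AimAt is true.
; Losing the enemy clears the rifle and fire-mode flags and closes the Gate.
; Pawn sensing is empty, and the older player-follow logic with debug prints is disconnected.
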(event `self.ReceiveBeginPlay`
  (`parent.ReceiveBeginPlay`))

(event `self.PawnSensing.OnSeePawn`
  (params (Pawn :type "Pawn Object Reference")))

(event `self.ReceiveTick`
  (params (DeltaSeconds :type "Float (single-precision)")))

(event `OnEnemyFound`
  (set `self.UseRifle` true)
  (set `self.FireMode` true)
  (`|ExecutionSequence`
    (:`then_0`
      (goto _label :!via `Open`))
    (:`then_1`
      (`/Engine/EditorBlueprintResources/StandardMacros.Gate` true :!label _label
        (:`Exit`
          (`|ExecutionSequence`
            (:`then_0`
              (if (`self.AimAt`)
                (set `self.Fire` true)
                (`KismetSystemLibrary.Delay` 0.5)
                (`self.FireBullet`)))
            (:`then_1`
              (`KismetSystemLibrary.RetriggerableDelay` 0.2)
              (goto _label))))))))

(event `OnEnemyLost`
  (set `self.UseRifle` false)
  (set `self.FireMode` false)
  (goto _label :!via `Close`))

(fn `UserConstructionScript`
  (`parent.UserConstructionScript`))