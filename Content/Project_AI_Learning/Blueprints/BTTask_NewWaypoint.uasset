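; Behavior Tree task that picks an AI character's target waypoint from a Route blackboard index.
; It first resets Route to zero if the value is at or below MaxRoute.
; It caches all BP_CharacterWaypoint actors, then writes the location of the one whose Position matches Route to TargetPoint.
; The task finishes as failed, with no success path.
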(event `self.ReceiveExecute`
  (params (OwnerActor :type "Actor Object Reference"))
  (`|ExecutionSequence`
    (:`then_0`
      (if (<= (`BTFunctionLibrary.GetBlackboardValueAsInt` (`self.Route`)) (`self.MaxRoute`))
        (`BTFunctionLibrary.SetBlackboardValueAsInt` (`self.Route`))))
    (:`then_1`
      (if (not (`KismetArrayLibrary.Array_IsNotEmpty` (`self.WaypointReferences`)))
        (bind _outactors (`GameplayStatics.GetAllActorsOfClass` "/Game/Project_AI_Learning/Blueprints/BP_CharacterWaypoint.BP_CharacterWaypoint_C"))
        (set `self.WaypointReferences` _outactors))
      (for _array_element (`self.WaypointReferences`)
        (if (== (`/Game/Project_AI_Learning/Blueprints/BP_CharacterWaypoint.Position` _array_element) (`BTFunctionLibrary.GetBlackboardValueAsInt` (`self.Route`)))
          (`BTFunctionLibrary.SetBlackboardValueAsVector` (`self.TargetPoint`) (`Actor.K2_GetActorLocation` _array_element))
          (break)))
      (`self.FinishExecute` false))))